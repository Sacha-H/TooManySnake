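; BP_Objet is a physics object that the player's magnet can suck in and consume.
; Aspire disables physics, and Tick pulls the cube toward the player's MagnetReference at constant speed while the magnet stays on.
; Switching the magnet off restores physics, collision and scale, unless a Sphere overlap has already committed it.
; That overlap keeps the pull active while a timeline shrinks the cube, then destroys the actor.
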(event OnComponentBeginOverlap(Sphere)
  (params (OverlappedComponent :type Primitive%20Component%20Object%20Reference) (OtherActor :type Actor%20Object%20Reference) (OtherComp :type Primitive%20Component%20Object%20Reference) (OtherBodyIndex :type Integer) (bFromSweep :type Boolean) (SweepResult :type Hit%20Result%20Structure%20%28by%20ref%29))
  (bind _cube (Variables|Default|GetCube))
  (Variables|Default|SetTooLate true)
  (bind _scaled (Timeline|Aspired4ever PlayFromStart)
    (:Update
      (Transformation|SetWorldScale3D _cube (Math|Vector|Lerp(Vector) (Transformation|GetWorldScale _cube) "0.000000,0.000000,0.000000" _scaled)))
    (:End
      (Development|PrintString "ASPIRED")
      (Actor|DestroyActor))))

(event EventTick
  (params (DeltaSeconds :type Float%20%28single-precision%29))
  (bind _cube (Variables|Default|GetCube))
  (if (Variables|Default|GetAspired)
    (bind _player_ref (Variables|Default|GetPlayer%20Ref)
      (:then
        (if (Variables|Default|GetTooLate)
          (Transformation|SetWorldLocation _cube (Math|Interpolation|VInterptoConstant (Transformation|GetWorldLocation _cube) (Transformation|GetWorldLocation (Variables|/Game/Tho/BP/BP_FirstPersonCharacter_Tho.BP_FirstPersonCharacter_Tho_C|GetMagnetReference _player_ref)) (Utilities|Time|GetWorldDeltaSeconds) 2.5e+02) false false :!label _label)
          (elif (Variables|/Game/Tho/BP/BP_FirstPersonCharacter_Tho.BP_FirstPersonCharacter_Tho_C|GetMagnetON? _player_ref)
            (goto _label)
            (else
              (Physics|SetSimulatePhysics (Variables|Default|GetCube) true)
              (Variables|Default|SetAspired false)
              (Transformation|SetWorldScale3D _cube (Variables|Default|GetWorldScale))
              (Collision|SetCollisionEnabled (Variables|Default|GetCube) "QueryAndPhysics")))))
      (:else))))

(event EventBeginPlay
  (bind _asbp_first_person_character_tho (Utilities|Casting|CastToBP_FirstPersonCharacter_Tho (Game|GetPlayerCharacter 0)))
  (Variables|Default|SetPlayer%20Ref _asbp_first_person_character_tho)
  (Variables|Default|SetWorldScale (Transformation|GetWorldScale (Variables|Default|GetCube))))

(event EventAspire
  (params (PlayerRef :type BP%20First%20Person%20Character%20Tho%20Object%20Reference) (Begin? :type Boolean))
  (if Begin?
    (Physics|SetSimulatePhysics (Variables|Default|GetCube) false)
    (Collision|SetCollisionEnabled (Variables|Default|GetCube) "QueryOnly")
    (Variables|Default|SetAspired true)))

(fn ConstructionScript)